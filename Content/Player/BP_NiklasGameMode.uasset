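; Game mode that handles player respawning at the last checkpoint.
; RespawnPlayer destroys the current character, spawns a fresh BP_TheFoolPlayer at the POS transform of LastCheckpoint, and has the player controller possess it.
; It then sets the new character's movement mode to Walking; BeginPlay, Tick and the construction script are empty.
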(event `Respawn Player`
  (bind (_returnvalue_location _returnvalue_rotation) (`KismetMathLibrary.BreakTransform` (`SceneComponent.K2_GetComponentToWorld` (`/Game/CheckpointSystem/BP_Checkpoint.POS` (`self.LastCheckpoint`)))))
  ; Respawn player
  (`self.K2_DestroyActor` (`GameplayStatics.GetPlayerCharacter` 0))
  (bind _returnvalue (`|SpawnActorFromClass` "/Game/Player/BP_TheFoolPlayer.BP_TheFoolPlayer_C" (`KismetMathLibrary.MakeTransform` _returnvalue_location _returnvalue_rotation) "AlwaysSpawn" "MultiplyWithRoot" null null))
  (`Controller.Possess` (`GameplayStatics.GetPlayerController` 0) _returnvalue)
  (bind _ascharacter (cast `Character` (`GameplayStatics.GetPlayerPawn` 0)))
  (`CharacterMovementComponent.SetMovementMode` (`Character.CharacterMovement` _ascharacter) "MOVE_Walking" 0))

(fn `UserConstructionScript`)