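; Player controller for BP_TheFoolPlayer that turns move input into camera-relative pawn movement.
; BeginPlay adds the Enhanced Input mapping context and caches the controlled pawn as BP_TheFoolPlayer.
; IA_Move stores the joystick value on trigger, cancel and completion.
; Each Tick consumes pending movement input, then applies the stored value along the camera boom's right and forward vectors.
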(event `self.ReceiveBeginPlay`
  ; Adds MainMappingContext with Enhanced Input to Controller
  (`EnhancedInputSubsystemInterface.AddMappingContext` (subsystem `EnhancedInputLocalPlayerSubsystem`) "/Game/Player/Input/MainMappingContext.MainMappingContext" 0 (struct))
  (bind _asbp_the_fool_player (cast `/Game/Player/BP_TheFoolPlayer` (`self.K2_GetPawn`)))
  (set `self.As BP The Fool Player` _asbp_the_fool_player))

(event `self.ReceiveTick`
  (params (DeltaSeconds :type "Float (single-precision)"))
  (bind (_joystickinput_x _joystickinput_y) (`KismetMathLibrary.BreakVector2D` (`self.JoystickInput`)))
  (bind _returnvalue (`self.K2_GetPawn` (`GameplayStatics.GetPlayerController` 0)))
  (bind _cameraboom (`InputCharacter.CameraBoom` (`self.As BP The Fool Player`)))
  ; Consumes Movement Input and Compensates for Camera Offset
  (bind _returnvalue_2 (`Pawn.ConsumeMovementInputVector` _returnvalue))
  (`Pawn.AddMovementInput` _returnvalue (+ (* (`SceneComponent.GetRightVector` _cameraboom) _joystickinput_x) (* (`SceneComponent.GetForwardVector` _cameraboom) _joystickinput_y)) 1.0 false))

(event `EnhancedInput|/Game/Player/Input/Actions/IA_Move`
  (params (ActionValue :type "Vector2D Structure") (ElapsedSeconds :type "Float (double-precision)") (TriggeredSeconds :type "Float (double-precision)") (InputAction :type "InputAction Object Reference" :default "/Game/Player/Input/Actions/IA_Move.IA_Move"))
  ; Consumes Movement Input and Compensates for Camera Offset
  (:`Triggered`
    (set `self.JoystickInput` ActionValue :!label _label))
  (:`Canceled`
    (goto _label))
  (:`Completed`
    (goto _label)))

(fn `UserConstructionScript`)