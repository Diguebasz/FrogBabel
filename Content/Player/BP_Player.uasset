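; BP_Player is the player Blueprint, handling an orbit-style camera and death with respawn.
; Each tick it aims the CameraBoom from the player toward a Center point on the horizontal plane, with a fixed downward pitch and a CameraOffsetAngle added to yaw.
; OnDeath turns the mesh into a physics body with collision, sets Dead, then reloads the current level after a short delay.
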(event `self.ReceiveBeginPlay`)

(event `self.ReceiveTick`
  (params (DeltaSeconds :type "Float (single-precision)"))
  (bind (_returnvalue_x _returnvalue_y _returnvalue_z) (`KismetMathLibrary.BreakVector` (`self.K2_GetActorLocation`)))
  (bind (_center_x _center_y) (`KismetMathLibrary.BreakVector` (`self.Center`)))
  (bind (_returnvalue_roll _returnvalue_pitch _returnvalue_yaw) (`KismetMathLibrary.BreakRotator` (`KismetMathLibrary.FindLookAtRotation` (`KismetMathLibrary.MakeVector` _returnvalue_x _returnvalue_y _returnvalue_z) (`KismetMathLibrary.MakeVector` _center_x _center_y _returnvalue_z))))
  ; Centered & offset camera
  (`|ExecutionSequence`
    (:`then_0`
      (`SceneComponent.K2_SetWorldRotation` (`self.CameraBoom`) (`KismetMathLibrary.MakeRotator` _returnvalue_roll -24.0 (+ _returnvalue_yaw (+ (`self.CameraOffsetAngle`) 0.0))) false false))))

(event `OnDeath`
  (bind _mesh (`self.Mesh`))
  ; Death & respawn
  (`PrimitiveComponent.SetSimulatePhysics` _mesh true)
  (`PrimitiveComponent.SetCollisionEnabled` _mesh "QueryAndPhysics")
  (set `self.Dead` true)
  (`KismetSystemLibrary.Delay` 3.0)
  (bind _returnvalue (`GameplayStatics.GetCurrentLevelName` true))
  (`GameplayStatics.OpenLevel` (`KismetStringLibrary.Conv_StringToName` _returnvalue)))

(fn `UserConstructionScript`)