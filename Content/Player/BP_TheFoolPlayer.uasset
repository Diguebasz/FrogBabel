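; Player character Blueprint for the Fool, handling an arena-style camera and a death and respawn loop with extra lives.
; Tick yaws the camera boom toward a Center point at fixed pitch, plus an adjustable offset angle.
; IsNotDead triggers OnDeath at zero health, which spends a life, ragdolls the mesh and calls Respawn after a delay.
; Respawn restores health at the last checkpoint; without spare lives the player just stays flagged dead.
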(event `CustomEvent`)

(event `self.ReceiveTick`
  (params (DeltaSeconds :type "Float (single-precision)"))
  (bind (_returnvalue_x _returnvalue_y _returnvalue_z) (`KismetMathLibrary.BreakVector` (`self.K2_GetActorLocation`)))
  (bind (_center_x _center_y) (`KismetMathLibrary.BreakVector` (`self.Center`)))
  (bind (_returnvalue_roll _returnvalue_pitch _returnvalue_yaw) (`KismetMathLibrary.BreakRotator` (`KismetMathLibrary.FindLookAtRotation` (`KismetMathLibrary.MakeVector` _returnvalue_x _returnvalue_y _returnvalue_z) (`KismetMathLibrary.MakeVector` _center_x _center_y _returnvalue_z))))
  ; Centered & offset camera
  (`|ExecutionSequence`
    (:`then_0`
      (`SceneComponent.K2_SetWorldRotation` (`self.CameraBoom`) (`KismetMathLibrary.MakeRotator` _returnvalue_roll -24.0 (+ _returnvalue_yaw (+ (`self.CameraOffsetAngle`) 0.0))) false false))))

(event `IsNotDead`
  ; Check if Player has more than 0 health
  (if (and (<= (`self.Health`) 0.0) (not (`self.Dead`)))
    (`self.OnDeath`)))

(event `OnDeath`
  (bind _mesh (`self.Mesh`))
  ; Death event
  (set `self.Dead` true)
  (if (>= (`self.ExtraLives`) 1)
    (set `self.ExtraLives` (- (`self.ExtraLives`) 1))
    (`PrimitiveComponent.SetSimulatePhysics` _mesh true)
    (`PrimitiveComponent.SetCollisionEnabled` _mesh "QueryAndPhysics")
    (set `self.Dead` true)
    (`KismetSystemLibrary.Delay` 3.0)
    (`self.Respawn`)))

(event `Respawn`
  (bind _mesh (`self.Mesh`))
  ; Respawn
  (`PrimitiveComponent.SetSimulatePhysics` _mesh false)
  (`KismetSystemLibrary.Delay` 0.1)
  (`self.K2_SetActorLocationAndRotation` (`self.LastCheckpoint`))
  (`PrimitiveComponent.SetCollisionEnabled` _mesh "QueryAndPhysics")
  (set `self.Dead` false)
  (set `self.Health` 100.0))

(fn `UserConstructionScript`)