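; BP_FlyCreature is an ambient flying creature that flees once when the player pawn enters its ScareZone.
; Flee also alerts every creature in its ScareGroup, then after a random delay plays a take-off montage and audio and sets InAir.
; A timeline, rate-scaled by Speed over spline length, moves the skeletal mesh rather than the actor along the spline, then destroys the actor at the end.
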(event `self.ReceiveBeginPlay`
  (`AudioComponent.Stop` (`self.Audio`)))

(event `self.ScareZone.OnComponentBeginOverlap`
  (params (OverlappedComponent :type "PrimitiveComponent Object Reference") (OtherActor :type "Actor Object Reference") (OtherComp :type "PrimitiveComponent Object Reference") (OtherBodyIndex :type Integer) (bFromSweep :type Boolean) (SweepResult :type "HitResult Structure (by ref)"))
  (if (== OtherActor (`GameplayStatics.GetPlayerPawn` 0))
    (`self.Flee`)))

(event `Flee`
  (bind _spline (`self.Spline`))
  (bind _skeletalmesh (`self.SkeletalMesh`))
  (`/Engine/EditorBlueprintResources/StandardMacros.DoOnce` false
    (:`Completed`
      (`|ExecutionSequence`
        (:`then_0`
          (for _array_element (`self.ScareGroup`)
            (bind _asbp_fly_creature (cast `/Game/Characters/Fly/BP_FlyCreature` _array_element))
            (`self.Flee` _asbp_fly_creature))
          (`KismetSystemLibrary.Delay` (* (`KismetMathLibrary.RandomFloat`) 0.75))
          (`|ExecutionSequence`
            (:`then_0`
              ; Scale the timeline speed with the length of the spline
              (`TimelineComponent.SetPlayRate` (`self.FlyTimeline`) (/ (`self.Speed`) (`SplineComponent.GetSplineLength` (`self.Spline`))))
              (bind (_direction _time) (`Timeline|FlyTimeline`)
                (:`Update`
                  ; Move the skeletal mesh and not the actor, because the spline would move with the actor. Cheap workaround but its OK
                  (`SceneComponent.K2_SetWorldLocation` _skeletalmesh (`SplineComponent.GetLocationAtTime` _spline _time "World" false) false false)
                  (`SceneComponent.K2_SetRelativeRotation` _skeletalmesh (`KismetMathLibrary.ComposeRotators` (`SplineComponent.GetRotationAtTime` _spline _time "Local" false) (struct :`Yaw` -90.0)) false false))
                (:`Finished`
                  ; Destroy when its at the end of the spline
                  (`self.K2_DestroyActor`))))
            (:`then_1`
              (`|PlayMontage` (`self.SkeletalMesh`) "/Game/Characters/Fly/Animations/AM_Fly_TakeOff.AM_Fly_TakeOff"
                (:`then`
                  (set `self.InAir` true))))
            (:`then_2`
              (`AudioComponent.Play` (`self.Audio`) 0.0))))))))

(fn `UserConstructionScript`)