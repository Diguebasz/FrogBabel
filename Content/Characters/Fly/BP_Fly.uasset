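; BP_Fly is a fly actor that gets scared into flight when the player's pawn enters its ScareZone.
; The first such overlap plays the take-off montage on the skeletal mesh and sets InAir immediately, without waiting for the montage to finish.
; While InAir is set, Tick moves the fly along its forward vector at FlySpeed without sweeping, and nothing in the graph stops or resets it.
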(event `self.ReceiveTick`
  (params (DeltaSeconds :type "Float (single-precision)"))
  (if (`self.InAir`)
    (`self.K2_SetActorLocation` (+ (* (`self.GetActorForwardVector`) (* DeltaSeconds (`self.FlySpeed`))) (`self.K2_GetActorLocation`)))))

(event `self.ReceiveBeginPlay`)

(event `self.ScareZone.OnComponentBeginOverlap`
  (params (OverlappedComponent :type "PrimitiveComponent Object Reference") (OtherActor :type "Actor Object Reference") (OtherComp :type "PrimitiveComponent Object Reference") (OtherBodyIndex :type Integer) (bFromSweep :type Boolean) (SweepResult :type "HitResult Structure (by ref)"))
  (if (== OtherActor (`GameplayStatics.GetPlayerPawn` 0))
    (`/Engine/EditorBlueprintResources/StandardMacros.DoOnce` false
      (:`Completed`
        (`|PlayMontage` (`self.SkeletalMesh`) "/Game/Characters/Fly/Animations/AM_Fly_TakeOff.AM_Fly_TakeOff"
          (:`then`
            (set `self.InAir` true)))))))

(fn `UserConstructionScript`)