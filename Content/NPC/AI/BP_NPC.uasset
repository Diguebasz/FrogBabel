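; BP_NPC is an NPC character with a customizable skeletal appearance and a death sequence in which it plays a frog get-eaten animation.
; The construction script assigns its CustomizableObjectInstance to the customizable skeletal component.
; The Kill event is guarded by DoOnce: it disables movement, stops the current montage, plays the get-eaten montage, waits for its returned length, then destroys the actor.
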(event `/Game/LevelPrototyping/TestingLogic/BPI_Killable.Kill`
  (`/Engine/EditorBlueprintResources/StandardMacros.DoOnce` false
    (:`Completed`
      (`CharacterMovementComponent.SetMovementMode` (`self.CharacterMovement`) "MOVE_None" 0)
      (`self.StopAnimMontage` null)
      (bind _returnvalue (`self.PlayAnimMontage` "/Game/Characters/Fish/Animation/AM_Frog_Get_Eaten.AM_Frog_Get_Eaten"))
      (`KismetSystemLibrary.Delay` _returnvalue)
      (`self.K2_DestroyActor`))))

(fn `UserConstructionScript`
  (set `CustomizableSkeletalComponent.CustomizableObjectInstance` (`self.Customizable Object Instance`) (`self.CustomizableSkeletal`)))