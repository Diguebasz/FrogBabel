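; BPC_WaterLevelFollow is a component that moves its owning actor along with the level's BP_RisingWater actor.
; On BeginPlay it finds the water actor and caches the owner's starting location.
; Every Tick it teleportlessly sets the owner to that start plus the water's absolute world location, without sweeping.
; The offset uses all three axes and the water's position itself rather than its change since start.
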(event `self.ReceiveBeginPlay`
  (bind _returnvalue (`GameplayStatics.GetActorOfClass` "/Game/LevelPrototyping/TestingLogic/BP_RisingWater.BP_RisingWater_C"))
  (set `self.Water` _returnvalue)
  (set `self.StartPosition` (`Actor.K2_GetActorLocation` (`self.GetOwner`))))

(event `self.ReceiveTick`
  (params (DeltaSeconds :type "Float (single-precision)"))
  (`Actor.K2_SetActorLocation` (`self.GetOwner`) (+ (`self.StartPosition`) (`Actor.K2_GetActorLocation` (`self.Water`))) false false))